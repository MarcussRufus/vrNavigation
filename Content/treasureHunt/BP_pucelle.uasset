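; BP_pucelle is a collectible pickup for the treasure hunt that spins continuously in the level.
; Tick adds a fixed yaw increment to the Pucelle component each frame, without scaling by delta time.
; When the player pawn overlaps the Box, it calls TreasureFind on the first TreasureHunt_BP actor found, plays the Djingle sound at Pucelle's location and destroys itself.
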(event `self.ReceiveTick`
  (params (DeltaSeconds :type "Float (single-precision)"))
  (`SceneComponent.K2_AddRelativeRotation` (`self.Pucelle`) (`KismetMathLibrary.MakeRotator` 0.0 0.0 (`self.increment`)) false false))

(event `self.Box.OnComponentBeginOverlap`
  (params (OverlappedComponent :type "PrimitiveComponent Object Reference") (OtherActor :type "Actor Object Reference") (OtherComp :type "PrimitiveComponent Object Reference") (OtherBodyIndex :type Integer) (bFromSweep :type Boolean) (SweepResult :type "HitResult Structure (by ref)"))
  (if (== OtherActor (`GameplayStatics.GetPlayerPawn` 0))
    (bind _outactors (`GameplayStatics.GetAllActorsOfClass` "/Game/treasureHunt/treasureHunt_BP.treasureHunt_BP_C"))
    (`/Game/treasureHunt/treasureHunt_BP.treasureFind` (`|GetArrayItem` _outactors))
    (`GameplayStatics.PlaySoundAtLocation` "/Game/treasureHunt/djingle.djingle" (`SceneComponent.K2_GetComponentLocation` (`self.Pucelle`)) (struct) 1.0 1.0 0.0 null null null)
    (`self.K2_DestroyActor`)))

(fn `UserConstructionScript`)