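; Treasure hunt manager that tracks how many treasures are found in the level.
; On BeginPlay it counts all BP_pucelle actors to set the total number of treasures.
; Its treasureFind event increments the found count and prints it with the number remaining as on-screen debug text.
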(event `self.ReceiveBeginPlay`
  (bind _outactors (`GameplayStatics.GetAllActorsOfClass` "/Game/treasureHunt/BP_pucelle.BP_pucelle_C"))
  (set `self.numberTreasures` (`KismetArrayLibrary.Array_Length` _outactors)))

(event `treasureFind`
  (bind _output_get (set `self.numberTreasuresFind` (+ (`self.numberTreasuresFind`) 1)))
  (`KismetSystemLibrary.PrintString` (`KismetStringLibrary.Concat_StrStr` (`KismetStringLibrary.Conv_IntToString` _output_get) " treasures find, " (`KismetStringLibrary.Conv_IntToString` (- (`self.numberTreasures`) (`self.numberTreasuresFind`))) "remain.")))

(fn `UserConstructionScript`)