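; BP_Poutre is a timed beam challenge actor with Start, Gravel and End components that react to player hits, identified by display name.
; Gravel hits count failures, show a "retry" widget and recolor surfaces until the player touches Start again.
; Start sets the timer only while failures are zero; End prints time (computed as start minus now) and failures once.
; Tick gathers player-tagged actors, but the widget-facing rotation is disconnected.
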(event `self.ReceiveBeginPlay`
  (set `self.Display name player` "player")
  (bind _asbp_step_widget (cast `/Game/Map1/Steps/BP_StepWidget` (`WidgetComponent.GetUserWidgetObject` (`self.Widget`)))
    (:`then`
      (set `self.As BP Step Widget` _asbp_step_widget))
    (:`CastFailed`
      (`KismetSystemLibrary.PrintString` "ERROR cast step widget"))))

(event `self.ReceiveTick`
  (params (DeltaSeconds :type "Float (single-precision)"))
  (bind _outactors (`GameplayStatics.GetAllActorsWithTag` "player")))

(event `self.gravel.OnComponentHit`
  (params (HitComponent :type "PrimitiveComponent Object Reference") (OtherActor :type "Actor Object Reference") (OtherComp :type "PrimitiveComponent Object Reference") (NormalImpulse :type "Vector Structure") (Hit :type "HitResult Structure (by ref)"))
  (if (`self.fell`)
    _
    (elif (`KismetStringLibrary.EqualEqual_StrStr` (`KismetSystemLibrary.GetDisplayName` OtherActor) (`self.Display name player`))
      (`KismetSystemLibrary.PrintString` "Rate")
      (set `self.fell` true)
      (`/Engine/EditorBlueprintResources/StandardMacros.IncrementInt` (`self.faillure number`)
        (:`  `
          (`SceneComponent.SetVisibility` (`self.Widget`) true false)
          (set `/Game/Map1/Steps/BP_StepWidget.stepwidget_text` "retry" (`self.As BP Step Widget`))
          (`PrimitiveComponent.SetMaterial` (`self.gravel`) 0 "/Game/Map1/Material/M_red.M_red")
          (`PrimitiveComponent.SetMaterial` (`self.start`) 0 "/Game/Map1/Material/M_green.M_green")))
      (else
        (`KismetSystemLibrary.PrintString` "Collision with something (gravel)")))))

(event `self.start.OnComponentHit`
  (params (HitComponent :type "PrimitiveComponent Object Reference") (OtherActor :type "Actor Object Reference") (OtherComp :type "PrimitiveComponent Object Reference") (NormalImpulse :type "Vector Structure") (Hit :type "HitResult Structure (by ref)"))
  (if (`KismetStringLibrary.EqualEqual_StrStr` (`KismetSystemLibrary.GetDisplayName` OtherActor) (`self.Display name player`))
    (`SceneComponent.SetVisibility` (`self.Widget`) false false)
    (set `self.fell` false)
    (if (== (`self.faillure number`) 0)
      (set `self.Time` (`KismetMathLibrary.Now`))
      (`PrimitiveComponent.SetMaterial` (`self.start`) 0 "/Game/StarterContent/Materials/M_Basic_Floor.M_Basic_Floor")
      (`PrimitiveComponent.SetMaterial` (`self.end`) 0 "/Game/Map1/Material/M_green.M_green")
      (`PrimitiveComponent.SetMaterial` (`self.gravel`) 0 "/Game/StarterContent/Materials/M_Basic_Floor.M_Basic_Floor"))
    (else
      (`KismetSystemLibrary.PrintString` "Collision with something (start)"))))

(event `self.end.OnComponentHit`
  (params (HitComponent :type "PrimitiveComponent Object Reference") (OtherActor :type "Actor Object Reference") (OtherComp :type "PrimitiveComponent Object Reference") (NormalImpulse :type "Vector Structure") (Hit :type "HitResult Structure (by ref)"))
  (if (`KismetStringLibrary.EqualEqual_StrStr` (`KismetSystemLibrary.GetDisplayName` OtherActor) (`self.Display name player`))
    (if (`self.fell`)
      _
      (elif (not (`self.finished`))
        (set `self.finished` true)
        (bind _output_get (set `self.duration` (- (`self.Time`) (`KismetMathLibrary.Now`))))
        (`KismetSystemLibrary.PrintString` (`KismetStringLibrary.Concat_StrStr` "time" (`KismetStringLibrary.Conv_IntToString` (`KismetMathLibrary.GetMinutes` _output_get)) "' " (`KismetStringLibrary.Conv_IntToString` (`KismetMathLibrary.GetSeconds` _output_get)) "''" "  failures:" (`KismetStringLibrary.Conv_IntToString` (`self.faillure number`))))
        (`PrimitiveComponent.SetMaterial` (`self.end`) 0 "/Game/StarterContent/Materials/M_Basic_Floor.M_Basic_Floor")))
    (else
      (`KismetSystemLibrary.PrintString` "Collision with something(end)"))))

(fn `UserConstructionScript`)