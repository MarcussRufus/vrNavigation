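; BP_Slalom is a timed slalom course with six cones, whose physics simulation is set from a variable on BeginPlay.
; Hitting Start with an actor whose display name is "player" stores the current time and swaps materials to turn End green.
; The first player hit on End prints the elapsed time, computed as start minus now, and a Hit value that these graphs never update.
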(event `self.ReceiveBeginPlay`
  (bind _physic (`self.physic`))
  (`PrimitiveComponent.SetSimulatePhysics` (`self.cone1`) _physic)
  (`PrimitiveComponent.SetSimulatePhysics` (`self.cone2`) _physic)
  (`PrimitiveComponent.SetSimulatePhysics` (`self.cone3`) _physic)
  (`PrimitiveComponent.SetSimulatePhysics` (`self.cone4`) _physic)
  (`PrimitiveComponent.SetSimulatePhysics` (`self.cone5`) _physic)
  (`PrimitiveComponent.SetSimulatePhysics` (`self.cone`) _physic)
  (set `self.Display name player` "player"))

(event `self.start.OnComponentHit`
  (params (HitComponent :type "PrimitiveComponent Object Reference") (OtherActor :type "Actor Object Reference") (OtherComp :type "PrimitiveComponent Object Reference") (NormalImpulse :type "Vector Structure") (Hit :type "HitResult Structure (by ref)"))
  (if (`KismetStringLibrary.EqualEqual_StrStr` (`KismetSystemLibrary.GetDisplayName` OtherActor) (`self.Display name player`))
    (set `self.Time` (`KismetMathLibrary.Now`))
    (`PrimitiveComponent.SetMaterial` (`self.start`) 0 "/Game/StarterContent/Materials/M_Basic_Floor.M_Basic_Floor")
    (`PrimitiveComponent.SetMaterial` (`self.end`) 0 "/Game/Map1/Material/M_green.M_green")
    (else
      (`KismetSystemLibrary.PrintString` "Collision with something (start)"))))

(event `self.end.OnComponentHit`
  (params (HitComponent :type "PrimitiveComponent Object Reference") (OtherActor :type "Actor Object Reference") (OtherComp :type "PrimitiveComponent Object Reference") (NormalImpulse :type "Vector Structure") (Hit :type "HitResult Structure (by ref)"))
  (if (`KismetStringLibrary.EqualEqual_StrStr` (`KismetSystemLibrary.GetDisplayName` OtherActor) (`self.Display name player`))
    (if (not (`self.finished`))
      (set `self.finished` true)
      (bind _output_get (set `self.duration` (- (`self.Time`) (`KismetMathLibrary.Now`))))
      (`KismetSystemLibrary.PrintString` (`KismetStringLibrary.Concat_StrStr` "time" (`KismetStringLibrary.Conv_IntToString` (`KismetMathLibrary.GetMinutes` _output_get)) "' " (`KismetStringLibrary.Conv_IntToString` (`KismetMathLibrary.GetSeconds` _output_get)) "'', " (`KismetStringLibrary.Conv_IntToString` (`self.hit`)) "hit"))
      (`PrimitiveComponent.SetMaterial` (`self.end`) 0 "/Game/StarterContent/Materials/M_Basic_Floor.M_Basic_Floor"))
    (else
      (`KismetSystemLibrary.PrintString` "Collision with something (end)"))))

(fn `UserConstructionScript`)