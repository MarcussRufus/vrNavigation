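; BP_StepStart is the starting step in Map1, labelling the start and prompting the player to slalom to the next point.
; On BeginPlay it runs the parent logic, then sets the text on the inherited step and next-step widget references.
; All other behaviour comes from the parent class, as the overlap and tick events are disabled stubs and construction only calls the parent.
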(event `self.ReceiveBeginPlay`
  (`parent.ReceiveBeginPlay`)
  (set `/Game/Map1/Steps/BP_StepWidget.stepwidget_text` "START!!" (`self.As BP Step Widget`))
  (set `/Game/Map1/Steps/BP_NextStepWidget.nextstep text` "slalom until here!" (`self.As BP Next Step Widget`)))

(fn `UserConstructionScript`
  (`parent.UserConstructionScript`))