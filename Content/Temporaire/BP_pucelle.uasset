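; BP_pucelle is a temporary-folder Blueprint that yaws its Pucelle component over time.
; While Sens is true, each Tick sets Modif to -1 and adds a relative yaw of Modif times Increment, without delta-time scaling.
; When world yaw leaves the -90 to 90 degree range, Sens flips to false and rotation stops, as the graph has no reverse branch.
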(event `self.ReceiveTick`
  (params (DeltaSeconds :type "Float (single-precision)"))
  (bind (_returnvalue_roll _returnvalue_pitch _returnvalue_yaw) (`KismetMathLibrary.BreakRotator` (`SceneComponent.K2_GetComponentRotation` (`self.Pucelle`))))
  (if (`self.sens`)
    (bind _output_get (set `self.modif` -1.0))
    (`SceneComponent.K2_AddRelativeRotation` (`self.Pucelle`) (`KismetMathLibrary.MakeRotator` 0.0 0.0 (* _output_get (`self.increment`))) false false)
    (if (or (> _returnvalue_yaw 90.0) (< _returnvalue_yaw -90.0))
      (set `self.sens` (not (`self.sens`))))))

(fn `UserConstructionScript`)